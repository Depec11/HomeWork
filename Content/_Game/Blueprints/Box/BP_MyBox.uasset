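; BP_MyBox is a scoring target actor that awards points when hit by a first-person projectile.
; On Hit, it matches the projectile by display-name substring, then calls AddPoint with its Score and OnTarget on player 0's BP_PlayerState before destroying itself.
; An IsLocal check runs but its result is unused, and a BP_GameMode DestroyBox call sits disconnected.
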(event `self.ReceiveHit`
  (params (MyComp :type "PrimitiveComponent Object Reference") (Other :type "Actor Object Reference") (OtherComp :type "PrimitiveComponent Object Reference") (bSelfMoved :type Boolean) (HitLocation :type "Vector Structure") (HitNormal :type "Vector Structure") (NormalImpulse :type "Vector Structure") (Hit :type "HitResult Structure (by ref)"))
  (`self.IsLocal`)
  (if (`KismetStringLibrary.Contains` (`KismetSystemLibrary.GetDisplayName` Other) "BP_FirstPersonProjectile")
    (bind _asbp_player_state (cast `/Game/_Game/Blueprints/Multiplayer/BP_PlayerState` (`Controller.PlayerState` (`GameplayStatics.GetPlayerController` 0))))
    (`/Game/_Game/Blueprints/Multiplayer/BP_PlayerState.AddPoint` _asbp_player_state (`self.Score`))
    (`/Game/_Game/Blueprints/Multiplayer/BP_PlayerState.OnTarget` _asbp_player_state)
    (`self.K2_DestroyActor`)))

(fn `IsLocal`
  (returns (isLocal :type Boolean))
  (return (`Controller.IsLocalPlayerController` (`GameplayStatics.GetPlayerController` 0))))

(fn `UserConstructionScript`)