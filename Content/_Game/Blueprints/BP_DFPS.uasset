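; BP_DFPS is a hit-reactive Blueprint that responds to first-person projectiles striking it.
; On Hit, it identifies projectiles by searching the other object's display name for BP_FirstPersonProjectile rather than casting.
; It then casts player controller 0's PlayerState to BP_PlayerState, reduces that state's HP by a fixed amount and calls OnTarget on it.
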(event `self.ReceiveHit`
  (params (MyComp :type "PrimitiveComponent Object Reference") (Other :type "Actor Object Reference") (OtherComp :type "PrimitiveComponent Object Reference") (bSelfMoved :type Boolean) (HitLocation :type "Vector Structure") (HitNormal :type "Vector Structure") (NormalImpulse :type "Vector Structure") (Hit :type "HitResult Structure (by ref)"))
  (if (`KismetStringLibrary.Contains` (`KismetSystemLibrary.GetDisplayName` Other) "BP_FirstPersonProjectile")
    (bind _asbp_player_state (cast `/Game/_Game/Blueprints/Multiplayer/BP_PlayerState` (`Controller.PlayerState` (`GameplayStatics.GetPlayerController` 0))))
    (`/Game/_Game/Blueprints/Multiplayer/BP_PlayerState.DecreaseHP` _asbp_player_state 10.0)
    (`/Game/_Game/Blueprints/Multiplayer/BP_PlayerState.OnTarget` _asbp_player_state)))

(fn `UserConstructionScript`
  (`parent.UserConstructionScript`))