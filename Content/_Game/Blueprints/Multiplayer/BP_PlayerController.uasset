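; Multiplayer player controller that requests a pawn for the local player on BeginPlay and again when R is pressed.
; The SR_SpawnPlayer event asks BP_GameMode to spawn a player for this controller, then possesses the returned pawn.
; Debug keys print the first player's ID and name, or their points from BP_PlayerState.
; A short BeginPlay timer fires an empty event.
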(event `self.ReceiveBeginPlay`
  (`parent.ReceiveBeginPlay`)
  (`KismetSystemLibrary.K2_SetTimerDelegate` (delegate `MyDelay`) 0.01)
  (bind _islocal (`self.IsLocal`))
  (if _islocal
    (`self.SR_SpawnPlayer`)))

(event `SR_SpawnPlayer`
  (bind _asbp_game_mode (cast `/Game/_Game/Blueprints/Multiplayer/BP_GameMode` (`GameplayStatics.GetGameMode`)))
  (bind _bp_firstpersoncharacter (`/Game/_Game/Blueprints/Multiplayer/BP_GameMode.SpawnPlayer` _asbp_game_mode self))
  (`self.Possess` self _bp_firstpersoncharacter))

(event `MyDelay`)

(event `Key|One`
  (params (Key :type "Key Structure"))
  (:`Pressed`
    (`self.ShowID` self)))

(event `Key|Two`
  (params (Key :type "Key Structure"))
  (:`Pressed`
    (bind _asbp_player_state (cast `/Game/_Game/Blueprints/Multiplayer/BP_PlayerState` (`Controller.PlayerState` (`GameplayStatics.GetPlayerController` 0))))
    (`KismetSystemLibrary.PrintString` (`KismetStringLibrary.Conv_DoubleToString` (`/Game/_Game/Blueprints/Multiplayer/BP_PlayerState.GetPoint` _asbp_player_state)) true true (struct :`G` 0.66 :`B` 1.0 :`A` 1.0) 600.0)))

(event `Key|R`
  (params (Key :type "Key Structure"))
  (:`Pressed`
    (`self.SR_SpawnPlayer`)))

(fn `IsLocal`
  (returns (isLocal :type Boolean))
  (return (`self.IsLocalPlayerController`)))

(fn `ShowID`
  (bind _playerstate (`Controller.PlayerState` (`GameplayStatics.GetPlayerController` 0)))
  (if (`self.IsLocalPlayerController` self)
    (`KismetSystemLibrary.PrintString` (`KismetStringLibrary.Concat_StrStr` (`KismetStringLibrary.Conv_IntToString` (`PlayerState.PlayerId` _playerstate)) "-" (`KismetSystemLibrary.GetDisplayName` _playerstate)) true true (struct :`G` 0.66 :`B` 1.0 :`A` 1.0) 600.0)))

(fn `UserConstructionScript`
  (`parent.UserConstructionScript`))