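; Multiplayer GameMode Blueprint that handles player spawning and a box-removal routine.
; SpawnPlayer destroys the controller's existing pawn and spawns a BP_DFPS at a random BP_PlayerInitPoint, returning it without possessing it.
; DestroyBox searches "BOX"-tagged actors by display name with debug prints; on a match it calls DestroyActor with no explicit target, so on itself.
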(fn `DestroyBox`
  (params (name :type String))
  (`KismetSystemLibrary.PrintString` "Hello")
  (bind _outactors (`GameplayStatics.GetAllActorsWithTag` "BOX"))
  (for _array_element _outactors
    (bind _returnvalue (`KismetSystemLibrary.GetDisplayName` _array_element))
    (`KismetSystemLibrary.PrintString` (`KismetStringLibrary.Concat_StrStr` _returnvalue "-" name))
    (if (`KismetStringLibrary.EqualEqual_StrStr` _returnvalue name)
      (`self.K2_DestroyActor`)
      (break))))

(fn `RandPlayerInitPos`
  (returns (transform :type "Transform Structure"))
  (bind _outactors (`GameplayStatics.GetAllActorsOfClass` "/Game/_Game/Blueprints/BP_PlayerInitPoint.BP_PlayerInitPoint_C"))
  (return (`self.GetTransform` (`|GetArrayItem` _outactors (`KismetMathLibrary.RandomIntegerInRange` 0 (- (`KismetArrayLibrary.Array_Length` _outactors) 1))))))

(fn `SpawnPlayer`
  (params (playerController :type "/Game/_Game/Blueprints/Multiplayer/BP_PlayerController Object Reference"))
  (returns (BP_FirstPersonCharacter :type "/Game/FirstPerson/Blueprints/BP_FirstPersonCharacter Object Reference"))
  (bind _returnvalue (`Controller.K2_GetPawn` playerController))
  (`/Engine/EditorBlueprintResources/StandardMacros.IsValid` _returnvalue
    (:`Is Valid`
      (`self.K2_DestroyActor` _returnvalue))
    (:`Is Not Valid`
      _))
  (bind _returnvalue_2 (`|SpawnActorFromClass` "/Game/_Game/Blueprints/BP_DFPS.BP_DFPS_C" (`self.RandPlayerInitPos`) "Undefined" "MultiplyWithRoot" null null))
  (return _returnvalue_2))

(fn `UserConstructionScript`
  (`parent.UserConstructionScript`))