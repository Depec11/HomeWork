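; BP_Monster is an enemy actor that rewards the player when shot and hurts the player on contact.
; Its Hit event identifies the other actor by matching substrings in its display name.
; A projectile hit adds points, calls OnTarget on the first player's BP_PlayerState and destroys the monster.
; A hit from BP_DFPS, apparently the player character, decreases HP on that same player state and leaves the monster alive.
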(event `self.ReceiveHit`
  (params (MyComp :type "PrimitiveComponent Object Reference") (Other :type "Actor Object Reference") (OtherComp :type "PrimitiveComponent Object Reference") (bSelfMoved :type Boolean) (HitLocation :type "Vector Structure") (HitNormal :type "Vector Structure") (NormalImpulse :type "Vector Structure") (Hit :type "HitResult Structure (by ref)"))
  (bind _returnvalue (`KismetSystemLibrary.GetDisplayName` Other))
  (if (`KismetStringLibrary.Contains` _returnvalue "BP_FirstPersonProjectile")
    (bind _asbp_player_state (cast `/Game/_Game/Blueprints/Multiplayer/BP_PlayerState` (`GameplayStatics.GetPlayerState` 0)))
    (`/Game/_Game/Blueprints/Multiplayer/BP_PlayerState.AddPoint` _asbp_player_state 5.0)
    (`/Game/_Game/Blueprints/Multiplayer/BP_PlayerState.OnTarget` _asbp_player_state)
    (`self.K2_DestroyActor`)
    (elif (`KismetStringLibrary.Contains` _returnvalue "BP_DFPS")
      (bind _asbp_player_state_2 (cast `/Game/_Game/Blueprints/Multiplayer/BP_PlayerState` (`GameplayStatics.GetPlayerState` 0)))
      (`/Game/_Game/Blueprints/Multiplayer/BP_PlayerState.DecreaseHP` _asbp_player_state_2 5.0))))

(fn `UserConstructionScript`)